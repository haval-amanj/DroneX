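; BP_SmallSphere is a short-lived moving sphere actor that scales into existence, flies and spins, then scales out and destroys itself.
; BeginPlay plays the wink-in timeline, picks a scaled random rotation rate and starts a four-second timer for the wink-out timeline.
; Tick moves the actor along its forward vector at Speed and applies the spin, both scaled by delta time, so the changing heading bends its path.
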(event Custom|WinkOut
  ;[0.15 0.01719 0.01719 0.5] WinkOut Sphere
  (bind _scaletrack (Timeline|WinkOutTimeline Play)
    (:Update
      (CallFunction|ScaleSphere _scaletrack))
    (:Finished
      (Actor|DestroyActor))))

(event Custom|WinkIn
  ;[0.15 0.01797 0.01797 0.5] Wink into Existence
  (bind _scale (Timeline|WinkInTimeline Play)
    (:Update
      (Transformation|SetWorldScale3D (Variables|Default|GetSM_SmallSphere) _scale))))

(event EventBeginPlay
  (CallFunction|Winkin)
  (Variables|SphereMovment|SetDelta%20Rotation (* (Math|Random|RandomRotator false) (Variables|SphereMovment|GetRotationScaleFactore)))
  ;[0.15 0.01719 0.01719 0.5] WinkOut Sphere
  (Utilities|Time|SetTimerbyEvent (delegate Custom|WinkOut) 4.0))

(event EventTick
  (params (DeltaSeconds :type Float%20%28single-precision%29))
  ;[0.000845 0.1313 0.15 0.5391] update Location and Rotation
  (CallFunction|UpdateLocation)
  (CallFunction|UpdateRotation))

(fn ConstructionScript)

(fn UpdateLocation
  (Transformation|AddActorWorldOffset (* (Transformation|GetActorForwardVector) (* (Utilities|Time|GetWorldDeltaSeconds) (Variables|SphereMovment|GetSpeed)))))

(fn UpdateRotation
  (Class|Actor|AddActorWorldRotation (* (Variables|SphereMovment|GetDelta%20Rotation) (Utilities|Time|GetWorldDeltaSeconds))))

(fn ScaleSphere
  (params (Scale :type Float%20%28single-precision%29))
  (Transformation|SetWorldScale3D (Variables|Default|GetSM_SmallSphere) (Math|Vector|MakeVector Scale Scale Scale)))