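; BP_BlasterBeam is a blaster beam actor that ends the game when it hits its target pawn.
; On BeginPlay it binds the BlasterBeam component's hit event to CheackHittingActor through a handler.
; Each hit spawns the NS_BeamBurst effect at the impact point, oriented along the surface normal.
; A hit on TargetPawn quits the game outright, while any other hit destroys the beam.
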(event Custom|OnBlasterBeamHit
  (params (HitComponent :type Primitive%20Component%20Object%20Reference) (OtherActor :type Actor%20Object%20Reference) (OtherComp :type Primitive%20Component%20Object%20Reference) (NormalImpulse :type Vector) (Hit :type Hit%20Result%20Structure%20%28by%20ref%29))
  (CallFunction|CheackHittingActor OtherActor Hit))

(event EventBeginPlay
  (Collision|BindEventtoOnComponentHit (Variables|Default|GetBlasterBeam) (delegate Custom|OnBlasterBeamHit)))

(fn ConstructionScript)

(fn CheackHittingActor
  (params (HittingActor :type Object%20Object%20Reference) (Hit :type Hit%20Result%20Structure%20%28by%20ref%29))
  (bind (_bblockinghit _binitialoverlap _time _distance _location _impactpoint _normal) (Collision|BreakHitResult Hit))
  (Niagara|SpawnSystematLocation "/Game/GameAssets/Assets/FX/NS_BeamBurst.NS_BeamBurst" _location (Math|Rotator|MakeRotfromX _normal))
  (if (== HittingActor (Variables|Default|GetTargetPawn))
    (Game|QuitGame 0 "Quit" false)
    (else
      (Actor|DestroyActor))))